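; Spline-based Blueprint that builds a deformed mesh along an editable spline, rebuilt by the Construction Script with no active runtime logic.
; It adds one Spline Mesh Component per segment, using the SplineMesh and ForwardAxis variables, and attaches it to the spline.
; Each segment takes local positions and tangents from neighboring spline points so pieces join continuously.
; Segments use query-only collision, commented as making the spline walkable.
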(event EventBeginPlay)

(event Collision|EventActorBeginOverlap
  (params (OtherActor :type Actor%20Object%20Reference)))

(event EventTick
  (params (DeltaSeconds :type Float%20%28single-precision%29)))

(fn ConstructionScript
  (bind _spline (Variables|Default|GetSpline))
  (for _index (range 0 (- (Spline|GetNumberOfSplinePoints _spline) 2)) ; Creates a loop so it continuously runs and checks
    ;[1 1 1] Finally gives the spline a mesh when placed and manipulated
    (bind _returnvalue (AddComponent|AddSplineMeshComponent false))
    (Components|StaticMesh|SetStaticMesh _returnvalue (Variables|Default|GetSplineMesh)) ; Gives the spline a mesh that is provided
    ;[1 1 1] Finds the axis then attaches the mesh to the spline to make sure it follows
    (SplineMesh|SetForwardAxis _returnvalue (Variables|Default|GetForwardAxis) true)
    (Transformation|AttachComponentToComponent _returnvalue _spline "None" "KeepRelative" "KeepRelative" "KeepRelative" true) ; This makes sure each spline body connects to the rest
    (SplineMesh|SetStartandEnd _returnvalue (Spline|GetLocationatSplinePoint _spline _index "Local") (Spline|GetTangentatSplinePoint _spline _index "Local") (Spline|GetLocationatSplinePoint _spline (+ _index 1) "Local") (Spline|GetTangentatSplinePoint _spline (+ _index 1) "Local") true :!class /Script/Engine.SplineMeshComponent) ; each location provides where the spline begins and ends, which allows for everything to connect
    (Collision|SetCollisionEnabled _returnvalue "QueryOnly") ; Allows the player to walk on the spline
  ))