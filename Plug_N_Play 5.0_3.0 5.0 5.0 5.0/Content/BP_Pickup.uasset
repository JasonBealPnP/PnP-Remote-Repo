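; Interactable pickup that grants the first-person character higher air control, then removes itself.
; On BeginPlay it applies an impulse to its RAGDOLLT component, and box overlap by the player toggles a prompt widget's visibility.
; Interact changes the character movement's air control settings, hides the actor, disables collision and destroys it after a short delay.
; An explosion emitter spawn is present but unconnected.
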(event OnComponentBeginOverlap(Box_col)
  (params (OverlappedComponent :type Primitive%20Component%20Object%20Reference) (OtherActor :type Actor%20Object%20Reference) (OtherComp :type Primitive%20Component%20Object%20Reference) (OtherBodyIndex :type Integer) (bFromSweep :type Boolean) (SweepResult :type Hit%20Result%20Structure%20%28by%20ref%29))
  (Utilities|Casting|CastToFirstPersonCharacter OtherActor)
  (Rendering|SetVisibility (Variables|Default|GetWidget) true false))

(event OnComponentEndOverlap(Box_col)
  (params (OverlappedComponent :type Primitive%20Component%20Object%20Reference) (OtherActor :type Actor%20Object%20Reference) (OtherComp :type Primitive%20Component%20Object%20Reference) (OtherBodyIndex :type Integer))
  (Utilities|Casting|CastToFirstPersonCharacter OtherActor)
  (Rendering|SetVisibility (Variables|Default|GetWidget) false false))

(event EventBeginPlay
  (Physics|AddImpulse (Variables|Default|GetRAGDOLL_T) "1000.000000,1000.000000,1000.000000" "None" true))

(event EventInteract
  (bind _asfirst_person_character (Utilities|Casting|CastToFirstPersonCharacter (Game|GetPlayerCharacter 0)))
  (Variables|/Script/Engine.CharacterMovementComponent|SetAirControl (Variables|/Script/Engine.Character|GetCharacterMovement _asfirst_person_character) 1.0)
  (Variables|/Script/Engine.CharacterMovementComponent|SetAirControlBoostMultiplier (Variables|/Script/Engine.Character|GetCharacterMovement _asfirst_person_character) 2.0)
  (Variables|/Script/Engine.CharacterMovementComponent|SetAirControlBoostVelocityThreshold (Variables|/Script/Engine.Character|GetCharacterMovement _asfirst_person_character) 25.0)
  (Rendering|SetActorHiddenInGame true)
  (Collision|SetActorEnableCollision false)
  (Utilities|FlowControl|Delay 1.0)
  (Actor|DestroyActor))

(fn ConstructionScript)