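; Flickering lamp actor that switches its light on and off at irregular intervals from BeginPlay onward.
; Flicker runs a fixed off/on sequence with randomized Delays between steps, mixing short and longer gaps, then calls itself to loop endlessly.
; TurnOff and TurnOn keep the visuals in sync by swapping the bulb material slot on the Light component between black and lit and toggling SpotLight visibility.
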(event Custom|Flicker
  (Utilities|FlowControl|Delay (Math|Random|RandomFloatinRange 0.3 0.5))
  (CallFunction|TurnOff)
  (Utilities|FlowControl|Delay (Math|Random|RandomFloatinRange 0.5 0.8))
  (CallFunction|Turnon)
  (Utilities|FlowControl|Delay (Math|Random|RandomFloatinRange 0.8 1.5))
  (CallFunction|TurnOff)
  (Utilities|FlowControl|Delay (Math|Random|RandomFloatinRange 0.1 0.3))
  (CallFunction|Turnon)
  (Utilities|FlowControl|Delay (Math|Random|RandomFloatinRange 0.8 1.5))
  (CallFunction|TurnOff)
  (Utilities|FlowControl|Delay (Math|Random|RandomFloatinRange 0.1 0.3))
  (CallFunction|Turnon)
  (CallFunction|Flicker))

(event Custom|Turn%20Off
  (Rendering|Material|SetMaterial (Variables|Default|GetLight) 3 "/Game/Materials/M_TrafficLight/M_TrafficLightBlack.M_TrafficLightBlack")
  (Rendering|SetVisibility (Variables|Default|GetSpotLight) false false))

(event Custom|Turn%20On
  (Rendering|Material|SetMaterial (Variables|Default|GetLight) 3 "/Game/Materials/M_LampLight/M_LampLightBulb.M_LampLightBulb")
  (Rendering|SetVisibility (Variables|Default|GetSpotLight) true false))

(event EventBeginPlay
  (Utilities|FlowControl|Delay (Math|Random|RandomFloatinRange 0.3 0.5))
  (CallFunction|TurnOff)
  (Utilities|FlowControl|Delay (Math|Random|RandomFloatinRange 0.5 0.8))
  (CallFunction|Turnon)
  (Utilities|FlowControl|Delay (Math|Random|RandomFloatinRange 0.8 1.5))
  (CallFunction|TurnOff)
  (Utilities|FlowControl|Delay (Math|Random|RandomFloatinRange 0.1 0.3))
  (CallFunction|Turnon)
  (Utilities|FlowControl|Delay (Math|Random|RandomFloatinRange 0.8 1.5))
  (CallFunction|TurnOff)
  (Utilities|FlowControl|Delay (Math|Random|RandomFloatinRange 0.1 0.3))
  (CallFunction|Turnon)
  (CallFunction|Flicker))

(fn ConstructionScript)