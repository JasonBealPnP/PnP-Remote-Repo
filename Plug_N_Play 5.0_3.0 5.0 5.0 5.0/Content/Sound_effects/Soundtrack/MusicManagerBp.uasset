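; MusicManagerBp is a music manager that plays the game soundtrack and switches between tracks on request.
; On BeginPlay it creates and starts a 2D sound for every TrackList entry at zero volume, then raises the IndexOfMusic track to MusicVolume.
; Change_Music mutes the current track, waits half a second and unmutes the chosen one, so all tracks keep running simultaneously and only volume changes.
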(event Custom|Change_Music
  (params (IndexofSongtoPlay :type Integer))
  (bind _soundtrack (Variables|Default|GetSoundtrack))
  (bind _output (Utilities|Array|Get(acopy) _soundtrack IndexofSongtoPlay))
  (Audio|Components|Audio|SetVolumeMultiplier (Variables|Default|GetCurrent%20Music%20Reference) 0.0 :!class /Script/Engine.AudioComponent)
  (Utilities|FlowControl|Delay 0.5)
  (Audio|Components|Audio|SetVolumeMultiplier _output (Variables|Default|GetMusic_Volume) :!class /Script/Engine.AudioComponent)
  (Variables|Default|SetCurrent%20Music%20Reference _output))

(event EventBeginPlay
  (bind _soundtrack (Variables|Default|GetSoundtrack))
  (bind _index_of_music (Variables|Default|GetIndex%20of%20Music))
  (bind _output (Utilities|Array|Get(acopy) _soundtrack _index_of_music))
  (for _array_element (Variables|Default|GetTrackList)
    (bind _returnvalue (Audio|CreateSound2D _array_element 1.0 1.0 0.0 0))
    (Utilities|Array|Add (Variables|Default|GetSoundtrack) _returnvalue)
    (Audio|Components|Audio|SetVolumeMultiplier _returnvalue 0.0 :!class /Script/Engine.AudioComponent)
    (Audio|Components|Audio|Play _returnvalue 0.0))
  (Audio|Components|Audio|SetVolumeMultiplier _output (Variables|Default|GetMusic_Volume) :!class /Script/Engine.AudioComponent)
  (Variables|Default|SetCurrent%20Music%20Reference _output))

(fn ConstructionScript)