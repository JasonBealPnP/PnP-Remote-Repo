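; ImpactBP is a short-lived actor, filed under impact particles, that turns to face the player and then removes itself.
; On BeginPlay it caches the FirstPersonCharacter and sets only its yaw from a look-at rotation toward that character, passed through a single RInterpTo call rather than updated per tick.
; It destroys itself after a two-second delay, but a failed cast skips both the rotation and the cleanup.
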(event EventBeginPlay
  (bind _asfirst_person_character (Utilities|Casting|CastToFirstPersonCharacter (Game|GetPlayerCharacter 0)))
  (Variables|Default|SetChara%20Ref _asfirst_person_character)
  (Transformation|SetActorRotation (Math|Rotator|MakeRotator 0.0 0.0 (.yaw (Math|Interpolation|RInterpTo (Transformation|GetActorRotation) (Math|Rotator|FindLookatRotation (Transformation|GetActorLocation) (Transformation|GetActorLocation (Variables|Default|GetChara%20Ref))) (Utilities|Time|GetWorldDeltaSeconds) 0.0))))
  (Utilities|FlowControl|Delay 2.0)
  (Actor|DestroyActor))

(event Collision|EventActorBeginOverlap
  (params (OtherActor :type Actor%20Object%20Reference)))

(event EventTick
  (params (DeltaSeconds :type Float%20%28single-precision%29)))

(fn ConstructionScript)