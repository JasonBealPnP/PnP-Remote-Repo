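; BP_laserBig is a laser actor with Niagara beam and impact effects, tinted in orange-red tones on BeginPlay.
; Each tick it line-traces forward on Visibility and feeds the hit point or trace end to the beam's LaserEnd parameter.
; The impact effect shows only at blocking hits.
; The beam length snaps to the hit distance, then grows over time up to a cap, so it visibly extends when unobstructed.
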(event EventBeginPlay
  (Effects|Components|ParticleSystem|SetColorParameter (Variables|Default|GetNiagaraLaser) "Color" "(R=1.000000,G=0.223360,B=0.000000,A=1.000000)")
  (Effects|Components|ParticleSystem|SetColorParameter (Variables|Default|GetNiagaraLaserImpact) "color" "(R=1.000000,G=0.329903,B=0.104484,A=1.000000)"))

(event Collision|EventActorBeginOverlap
  (params (OtherActor :type Actor%20Object%20Reference)))

(event EventTick
  (params (DeltaSeconds :type Float%20%28single-precision%29))
  (bind _returnvalue (Transformation|GetActorLocation))
  (Utilities|FlowControl|Sequence
    (:then_0
      (Variables|Default|SetTraceEnd (+ _returnvalue (* (Transformation|GetActorForwardVector) (Variables|Default|GetDistance))))
      (bind _outhit (Collision|LineTraceByChannel _returnvalue (+ _returnvalue (* (Transformation|GetActorForwardVector) (Variables|Default|GetDistance))) "TraceTypeQuery1" false 0 "None"))
      (Variables|Default|SetOut%20Hit%20Blocking%20Hit (.bblockinghit _outhit))
      (Variables|Default|SetOut%20Hit%20Location (.location _outhit))
      (Niagara|SetNiagaraVariable(Vector3) (Variables|Default|GetNiagaraLaser) "LaserEnd" (select (Variables|Default|GetOut%20Hit%20Blocking%20Hit) (Variables|Default|GetOut%20Hit%20Location) (Variables|Default|GetTraceEnd)))
      (Rendering|SetVisibility (Variables|Default|GetNiagaraLaserImpact) (Variables|Default|GetOut%20Hit%20Blocking%20Hit) false)
      (Transformation|SetWorldLocation (Variables|Default|GetNiagaraLaserImpact) (Variables|Default|GetOut%20Hit%20Location) false false)
      (if (Variables|Default|GetOut%20Hit%20Blocking%20Hit)
        (Variables|Default|SetDistance (Math|Vector|VectorLength (- (Variables|Default|GetOut%20Hit%20Location) (Transformation|GetActorLocation))))))
    (:then_1
      (if (< (Variables|Default|GetDistance) 5e+03)
        (Variables|Default|SetDistance (+ (Variables|Default|GetDistance) (* DeltaSeconds 2e+03)))))))

(fn ConstructionScript)