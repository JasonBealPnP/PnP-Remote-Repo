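; BloodSplatBP is a blood splatter actor that turns Niagara particle data into blood stain decals.
; On BeginPlay it registers itself as the Niagara system's callback object for two user parameters, so exported particle data returns to the Blueprint.
; For each received particle, a low-probability roll spawns a decal at its position, oriented against its velocity, which fades out after a short delay.
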(event EventBeginPlay
  (bind _self self)
  (bind _niagara (Variables|Default|GetNiagara))
  (Niagara|SetNiagaraVariable(Object) _niagara "User.BPCallBack" _self)
  (Niagara|SetNiagaraVariable(Object) _niagara "User.DropletSplash" _self))

(event Collision|EventActorBeginOverlap
  (params (OtherActor :type Actor%20Object%20Reference)))

(event EventTick
  (params (DeltaSeconds :type Float%20%28single-precision%29)))

(event EventParticleData
  (params (Data :type Array%20of%20Basic%20Particle%20Data%20Structures) (NiagaraSystem :type Niagara%20System%20Object%20Reference))
  (for _array_element Data
    (Variables|Default|SetSpawn (Math|Random|RandomBoolwithWeight 0.1))
    (if (Variables|Default|GetSpawn)
      (bind _returnvalue (Rendering|Decal|SpawnDecalatLocation "/Game/Particles/ParticleMiscMats/MS_Blood/Decal/010_Blood_Stain_sgfjdepc/010_Blood_Stain_sgfjdepc_8K_inst.010_Blood_Stain_sgfjdepc_8K_inst" "20.000000,40.000000,40.000000" (.Position (Utilities|Struct|BreakBasicParticleData _array_element)) (Math|Conversions|RotationFromXVector (* (.Velocity (Utilities|Struct|BreakBasicParticleData _array_element)) "-1.000000,-1.000000,-1.000000")) 0.0))
      (Rendering|Components|Decal|SetFadeOut _returnvalue 1.0 2.0 true))))

(fn ConstructionScript)